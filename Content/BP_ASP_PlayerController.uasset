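; BP_ASP_PlayerController is a player controller that turns Enhanced Input movement actions into movement of the controlled pawn.
; On BeginPlay it adds an input mapping context to the local player subsystem.
; The vertical and horizontal move actions feed their values as world-space X and Y vectors into the pawn's movement component, so movement follows world axes rather than camera or pawn rotation.
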(event Input|EnhancedActionEvents|EnhancedInputActionIA_ASP_MoveVertical
  (params (ActionValue :type Float%20%28double-precision%29) (ElapsedSeconds :type Float%20%28double-precision%29) (TriggeredSeconds :type Float%20%28double-precision%29) (InputAction :type Input%20Action%20Object%20Reference :default "/AdvancedSight/IA_ASP_MoveVertical.IA_ASP_MoveVertical"))
  (Class|PawnMovementComponent|AddInputVector (Pawn|GetMovementComponent (Pawn|GetControlledPawn)) (Math|Vector|MakeVector ActionValue 0.0 0.0) false))

(event Input|EnhancedActionEvents|EnhancedInputActionIA_ASP_MoveHorizontal
  (params (ActionValue :type Float%20%28double-precision%29) (ElapsedSeconds :type Float%20%28double-precision%29) (TriggeredSeconds :type Float%20%28double-precision%29) (InputAction :type Input%20Action%20Object%20Reference :default "/AdvancedSight/IA_ASP_MoveHorizontal.IA_ASP_MoveHorizontal"))
  (Class|PawnMovementComponent|AddInputVector (Pawn|GetMovementComponent (Pawn|GetControlledPawn)) (Math|Vector|MakeVector 0.0 ActionValue 0.0) false))

(event EventBeginPlay
  (Input|AddMappingContext (PlayerController|LocalPlayerSubsystems|GetEnhancedInputLocalPlayerSubsystem) (Variables|Default|GetInputMapping) 0 "(bIgnoreAllPressedKeysUntilRelease=True,bForceImmediately=False,bNotifyUserSettings=False)"))

(event EventTick
  (params (DeltaSeconds :type Float%20%28single-precision%29)))

(fn ConstructionScript)