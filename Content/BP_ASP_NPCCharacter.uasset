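; BP_ASP_NPCCharacter is an NPC character Blueprint that holds a patrol route as an array of points.
; GetCurrentPatrolPoint returns the point at the current index.
; NextPatrolPoint advances the index with modulo wraparound, looping the route, and returns the new point when the array is not empty.
; The event graph has only disabled default events, so movement is not driven here.
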(event EventBeginPlay
  (|CallParentFunction) ; This node is disabled and will not be called.\nDrag off pins to build functionality.
)

(event Collision|EventActorBeginOverlap
  (params (OtherActor :type Actor%20Object%20Reference))
  (|CallParentFunction OtherActor) ; This node is disabled and will not be called.\nDrag off pins to build functionality.
)

(event EventTick
  (params (DeltaSeconds :type Float%20%28single-precision%29))
  (|CallParentFunction DeltaSeconds) ; This node is disabled and will not be called.\nDrag off pins to build functionality.
)

(fn ConstructionScript
  (|CallParentFunction))

(fn GetCurrentPatrolPoint
  (return (Utilities|Array|Get(acopy) (Variables|Default|GetPatrolPoints) (Variables|Default|GetCurrentPatrolPointIndex))))

(fn NextPatrolPoint
  (if (> (Utilities|Array|Length (Variables|Default|GetPatrolPoints)) 0)
    (bind _output_get (Variables|Default|SetCurrentPatrolPointIndex (Math|Integer|%(Integer) (+ (Variables|Default|GetCurrentPatrolPointIndex) 1) (Utilities|Array|Length (Variables|Default|GetPatrolPoints)))))
    (return (Utilities|Array|Get(acopy) (Variables|Default|GetPatrolPoints) _output_get))
    (else
      (return 0))))