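; BP_ASP_AIController is an AI controller that runs the behavior tree assigned on the possessed BP_ASP_Character.
; AdvancedSight events drive the blackboard: perceiving a target stores it as the target actor.
; Losing the target clears it and records its location as last known, and forgetting it clears that location.
; The spotted event is unused.
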(event OnTargetSpotted(AdvancedSight)
  (params (TargetActor :type Actor%20Object%20Reference)))

(event OnTargetPerceived(AdvancedSight)
  (params (TargetActor :type Actor%20Object%20Reference))
  (bind _returnvalue (AI|GetBlackboard 0))
  (Utilities|IsValid _returnvalue
    (:Is%20Valid
      (AI|Components|Blackboard|SetValueasObject _returnvalue (Variables|Default|GetTargetActorKeyName) TargetActor))))

(event OnTargetLost(AdvancedSight)
  (params (TargetActor :type Actor%20Object%20Reference))
  (bind _returnvalue (AI|GetBlackboard 0))
  (Utilities|IsValid _returnvalue
    (:Is%20Valid
      (AI|Components|Blackboard|ClearValue _returnvalue (Variables|Default|GetTargetActorKeyName))
      (AI|Components|Blackboard|SetValueasVector (AI|GetBlackboard 0) (Variables|Default|GetLastKnownLocationKeyName) (Transformation|GetActorLocation TargetActor)))))

(event OnTargetForgot(AdvancedSight)
  (params (TargetActor :type Actor%20Object%20Reference))
  (bind _returnvalue (AI|GetBlackboard 0))
  (Utilities|IsValid _returnvalue
    (:Is%20Valid
      (AI|Components|Blackboard|ClearValue _returnvalue (Variables|Default|GetLastKnownLocationKeyName)))))

(event EventPossess
  (params (PossessedPawn :type Pawn%20Object%20Reference))
  (bind _asbp_asp_character (Utilities|Casting|CastToBP_ASP_Character PossessedPawn))
  (Utilities|IsValid (Variables|/AdvancedSight/BP_ASP_Character.BP_ASP_Character_C|GetBehaviorTree _asbp_asp_character)
    (:Is%20Valid
      (AI|RunBehaviorTree (Variables|/AdvancedSight/BP_ASP_Character.BP_ASP_Character_C|GetBehaviorTree _asbp_asp_character)))))

(fn ConstructionScript)